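; Toll booth road prop in Toon City with four independently animated pivots, which by the asset name are likely barrier arms.
; Each of the four collision components plays its own timeline on begin overlap, pitching the matching pivot by the track value times a shared Angle.
; On end overlap it waits a shared Delay, then reverses the timeline to return the pivot.
; Overlaps are not filtered by actor.
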(event OnComponentBeginOverlap(Collision_1A)
  (params (OverlappedComponent :type Primitive%20Component%20Object%20Reference) (OtherActor :type Actor%20Object%20Reference) (OtherComp :type Primitive%20Component%20Object%20Reference) (OtherBodyIndex :type Integer) (bFromSweep :type Boolean) (SweepResult :type Hit%20Result%20Structure%20%28by%20ref%29))
  (bind _newtrack_0 (Timeline|Timeline_0 Play)
    (:Update
      (Transformation|SetRelativeRotation (Variables|Default|GetPivot_1A) (Math|Rotator|MakeRotator 0.0 (* _newtrack_0 (Variables|Default|GetAngle)) 0.0) false false))))

(event OnComponentEndOverlap(Collision_1A)
  (params (OverlappedComponent :type Primitive%20Component%20Object%20Reference) (OtherActor :type Actor%20Object%20Reference) (OtherComp :type Primitive%20Component%20Object%20Reference) (OtherBodyIndex :type Integer))
  (Utilities|FlowControl|Delay (Variables|Default|GetDelay))
  (bind _newtrack_0 (Timeline|Timeline_0 Reverse)
    (:Update
      (Transformation|SetRelativeRotation (Variables|Default|GetPivot_1A) (Math|Rotator|MakeRotator 0.0 (* _newtrack_0 (Variables|Default|GetAngle)) 0.0) false false))))

(event OnComponentBeginOverlap(Collision_1B)
  (params (OverlappedComponent :type Primitive%20Component%20Object%20Reference) (OtherActor :type Actor%20Object%20Reference) (OtherComp :type Primitive%20Component%20Object%20Reference) (OtherBodyIndex :type Integer) (bFromSweep :type Boolean) (SweepResult :type Hit%20Result%20Structure%20%28by%20ref%29))
  (bind _newtrack_0 (Timeline|Timeline_1 Play)
    (:Update
      (Transformation|SetRelativeRotation (Variables|Default|GetPivot_1B) (Math|Rotator|MakeRotator 0.0 (* _newtrack_0 (Variables|Default|GetAngle)) 0.0) false false))))

(event OnComponentEndOverlap(Collision_1B)
  (params (OverlappedComponent :type Primitive%20Component%20Object%20Reference) (OtherActor :type Actor%20Object%20Reference) (OtherComp :type Primitive%20Component%20Object%20Reference) (OtherBodyIndex :type Integer))
  (Utilities|FlowControl|Delay (Variables|Default|GetDelay))
  (bind _newtrack_0 (Timeline|Timeline_1 Reverse)
    (:Update
      (Transformation|SetRelativeRotation (Variables|Default|GetPivot_1B) (Math|Rotator|MakeRotator 0.0 (* _newtrack_0 (Variables|Default|GetAngle)) 0.0) false false))))

(event OnComponentBeginOverlap(Collision_1D)
  (params (OverlappedComponent :type Primitive%20Component%20Object%20Reference) (OtherActor :type Actor%20Object%20Reference) (OtherComp :type Primitive%20Component%20Object%20Reference) (OtherBodyIndex :type Integer) (bFromSweep :type Boolean) (SweepResult :type Hit%20Result%20Structure%20%28by%20ref%29))
  (bind _newtrack_0 (Timeline|Timeline_3 Play)
    (:Update
      (Transformation|SetRelativeRotation (Variables|Default|GetPivot_1D) (Math|Rotator|MakeRotator 0.0 (* _newtrack_0 (Variables|Default|GetAngle)) 0.0) false false))))

(event OnComponentEndOverlap(Collision_1D)
  (params (OverlappedComponent :type Primitive%20Component%20Object%20Reference) (OtherActor :type Actor%20Object%20Reference) (OtherComp :type Primitive%20Component%20Object%20Reference) (OtherBodyIndex :type Integer))
  (Utilities|FlowControl|Delay (Variables|Default|GetDelay))
  (bind _newtrack_0 (Timeline|Timeline_3 Reverse)
    (:Update
      (Transformation|SetRelativeRotation (Variables|Default|GetPivot_1D) (Math|Rotator|MakeRotator 0.0 (* _newtrack_0 (Variables|Default|GetAngle)) 0.0) false false))))

(event OnComponentBeginOverlap(Collision_1C)
  (params (OverlappedComponent :type Primitive%20Component%20Object%20Reference) (OtherActor :type Actor%20Object%20Reference) (OtherComp :type Primitive%20Component%20Object%20Reference) (OtherBodyIndex :type Integer) (bFromSweep :type Boolean) (SweepResult :type Hit%20Result%20Structure%20%28by%20ref%29))
  (bind _newtrack_0 (Timeline|Timeline_2 Play)
    (:Update
      (Transformation|SetRelativeRotation (Variables|Default|GetPivot_1C) (Math|Rotator|MakeRotator 0.0 (* _newtrack_0 (Variables|Default|GetAngle)) 0.0) false false))))

(event OnComponentEndOverlap(Collision_1C)
  (params (OverlappedComponent :type Primitive%20Component%20Object%20Reference) (OtherActor :type Actor%20Object%20Reference) (OtherComp :type Primitive%20Component%20Object%20Reference) (OtherBodyIndex :type Integer))
  (Utilities|FlowControl|Delay (Variables|Default|GetDelay))
  (bind _newtrack_0 (Timeline|Timeline_2 Reverse)
    (:Update
      (Transformation|SetRelativeRotation (Variables|Default|GetPivot_1C) (Math|Rotator|MakeRotator 0.0 (* _newtrack_0 (Variables|Default|GetAngle)) 0.0) false false))))

(fn ConstructionScript)