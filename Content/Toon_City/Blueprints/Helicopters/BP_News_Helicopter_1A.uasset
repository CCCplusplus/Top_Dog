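; News helicopter prop Blueprint for Toon City with spinning main and tail rotors.
; The construction script maps the RotorRPM setting (off, low or high) to a speed value.
; On BeginPlay, that speed drives two RotatingMovement components on different axes, one updating the main rotor component and the other a tail rotor pivot.
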(event EventBeginPlay
  (bind _t (Variables|Default|Gett))
  (Variables|/Script/Engine.RotatingMovementComponent|SetRotationRate (Variables|Default|GetRotatingMovement_MainRotor) (Math|Rotator|MakeRotator 0.0 0.0 (Math|Conversions|ToFloat(Integer) _t)))
  (Variables|/Script/Engine.RotatingMovementComponent|SetRotationRate (Variables|Default|GetRotatingMovement_TailRotor) (Math|Rotator|MakeRotator (Math|Conversions|ToFloat(Integer) _t) 0.0 0.0))
  (Components|Movement|SetUpdatedComponent (Variables|Default|GetRotatingMovement_MainRotor) (Variables|Default|GetNews_Helicopter_1A_Main_Rotor_1A))
  (Components|Movement|SetUpdatedComponent (Variables|Default|GetRotatingMovement_TailRotor) (Variables|Default|GetTail_Rotor_Pivot)))

(fn ConstructionScript
  (switch Utilities|FlowControl|Switch|SwitchonE_HeloRotorSpeeds (Variables|Default|GetRotor%20RPM)
    (:NewEnumerator0
      (Variables|Default|Sett 0))
    (:NewEnumerator1
      (Variables|Default|Sett 300))
    (:NewEnumerator2
      (Variables|Default|Sett 3000))))