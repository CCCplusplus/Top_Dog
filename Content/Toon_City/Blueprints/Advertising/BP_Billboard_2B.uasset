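; BP_Billboard_2B is a Toon City advertising billboard with a rotating part.
; The construction script maps the BillboardRPM setting (off, low or high) to a rotation speed.
; On BeginPlay, that speed sets a single-axis rate on the BillboardRotator component, which is then pointed at the rotating billboard component.
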(event EventBeginPlay
  (bind _billboard_rotator (Variables|Default|GetBillboard%20Rotator))
  (Variables|/Script/Engine.RotatingMovementComponent|SetRotationRate _billboard_rotator (Math|Rotator|MakeRotator 0.0 0.0 (Math|Conversions|ToFloat(Integer) (Variables|Default|Gett))))
  (Components|Movement|SetUpdatedComponent _billboard_rotator (Variables|Default|GetBillboard_2B_Rotating_Billboard_2B)))

(fn ConstructionScript
  (switch Utilities|FlowControl|Switch|SwitchonE_HeloRotorSpeeds (Variables|Default|GetBillboard%20RPM)
    (:NewEnumerator0
      (Variables|Default|Sett 0))
    (:NewEnumerator1
      (Variables|Default|Sett 10))
    (:NewEnumerator2
      (Variables|Default|Sett 40))))