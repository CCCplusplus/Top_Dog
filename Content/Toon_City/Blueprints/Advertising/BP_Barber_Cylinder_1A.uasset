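; Barber pole advertising prop for Toon City whose center cylinder spins at a selectable speed.
; The construction script maps the CylinderRPM setting (off, low or high) to a speed value T, which is in degrees per second despite the RPM name.
; On BeginPlay, T sets a single-axis rotation rate on CylinderRotator, which then targets only the center mesh as its updated component.
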(event EventBeginPlay
  (bind _cylinder_rotator (Variables|Default|GetCylinder%20Rotator))
  (Variables|/Script/Engine.RotatingMovementComponent|SetRotationRate _cylinder_rotator (Math|Rotator|MakeRotator 0.0 0.0 (Math|Conversions|ToFloat(Integer) (Variables|Default|Gett))))
  (Components|Movement|SetUpdatedComponent _cylinder_rotator (Variables|Default|GetBarber_Cylinder_1A_Barber_Cylinder_1A_Center)))

(fn ConstructionScript
  (switch Utilities|FlowControl|Switch|SwitchonE_HeloRotorSpeeds (Variables|Default|GetCylinder%20RPM)
    (:NewEnumerator0
      (Variables|Default|Sett 0))
    (:NewEnumerator1
      (Variables|Default|Sett 30))
    (:NewEnumerator2
      (Variables|Default|Sett 60))))