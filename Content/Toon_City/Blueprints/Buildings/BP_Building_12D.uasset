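; Toon City building Blueprint with a door that spins continuously around a pivot at a selectable speed.
; The construction script maps the DoorRPM setting (off, low or high) to a speed value T.
; On BeginPlay, the negated T becomes the single-axis rotation rate of DoorRotator, which takes DoorPivot as its updated component so the movement component turns only the door.
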(event EventBeginPlay
  (bind _door_rotator (Variables|Default|GetDoor%20Rotator))
  (Variables|/Script/Engine.RotatingMovementComponent|SetRotationRate _door_rotator (Math|Rotator|MakeRotator 0.0 0.0 (Math|Conversions|ToFloat(Integer) (* (Variables|Default|Gett) -1))))
  (Components|Movement|SetUpdatedComponent _door_rotator (Variables|Default|GetDoor_Pivot)))

(fn ConstructionScript
  (switch Utilities|FlowControl|Switch|SwitchonE_HeloRotorSpeeds (Variables|Default|GetDoor%20RPM)
    (:NewEnumerator0
      (Variables|Default|Sett 0))
    (:NewEnumerator1
      (Variables|Default|Sett 20))
    (:NewEnumerator2
      (Variables|Default|Sett 80))))