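; Toon City building Blueprint with a cone that can spin at a selectable speed.
; The construction script maps the ConeRPM setting (off, low or high) to a rotation rate value.
; On BeginPlay, that value sets a single-axis rate on the RotatorCone component, which is pointed at PivotCone so it rotates that component without any Tick logic.
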(event EventBeginPlay
  (bind _rotator_cone (Variables|Default|GetRotator%20Cone))
  (Variables|/Script/Engine.RotatingMovementComponent|SetRotationRate _rotator_cone (Math|Rotator|MakeRotator 0.0 0.0 (Math|Conversions|ToFloat(Integer) (Variables|Default|Gett))))
  (Components|Movement|SetUpdatedComponent _rotator_cone (Variables|Default|GetPivot_Cone)))

(fn ConstructionScript
  (switch Utilities|FlowControl|Switch|SwitchonE_HeloRotorSpeeds (Variables|Default|GetCone%20RPM)
    (:NewEnumerator0
      (Variables|Default|Sett 0))
    (:NewEnumerator1
      (Variables|Default|Sett 20))
    (:NewEnumerator2
      (Variables|Default|Sett 80))))