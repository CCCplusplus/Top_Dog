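; BP_Window_Washer_1A is an industrial Toon City prop of a window washer rig whose cage hangs at an adjustable height.
; It sets the Cage bone of a PoseableMesh in component space, changing only Z to the negative absolute CageHeight so the value always points downward.
; The same logic runs in the Construction Script and again on BeginPlay, so the placed pose also applies at game start.
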(event EventBeginPlay
  (bind _poseablemesh (Variables|Default|GetPoseableMesh))
  (bind _returnvalue (Class|PoseableMeshComponent|GetBoneTransformbyName _poseablemesh "Cage" "ComponentSpace"))
  (Components|PoseableMesh|SetBoneTransformbyName _poseablemesh "Cage" (Math|Transform|MakeTransform (Math|Vector|MakeVector (.x (.location _returnvalue)) (.y (.location _returnvalue)) (Math|Conversions|ToFloat(Integer) (* (Math|Integer|Absolute(Integer) (Variables|Default|GetCage%20Height)) -1))) (.rotation _returnvalue) (.scale _returnvalue)) "ComponentSpace"))

(fn ConstructionScript
  (bind _poseablemesh (Variables|Default|GetPoseableMesh))
  (bind _returnvalue (Class|PoseableMeshComponent|GetBoneTransformbyName _poseablemesh "Cage" "ComponentSpace"))
  (Components|PoseableMesh|SetBoneTransformbyName _poseablemesh "Cage" (Math|Transform|MakeTransform (Math|Vector|MakeVector (.x (.location _returnvalue)) (.y (.location _returnvalue)) (Math|Conversions|ToFloat(Integer) (* (Math|Integer|Absolute(Integer) (Variables|Default|GetCage%20Height)) -1))) (.rotation _returnvalue) (.scale _returnvalue)) "ComponentSpace"))