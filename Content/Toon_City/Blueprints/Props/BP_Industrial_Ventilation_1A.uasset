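; Industrial ventilation prop for the Toon City set with four fans that spin at a selectable speed.
; The Construction Script converts the FanRPM setting (off, low or high) into a rotation rate.
; On BeginPlay, four rotator movement components apply that rate on a single axis, each bound to its own fan pivot, so the fans only start turning during play.
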(event EventBeginPlay
  (bind _t (Variables|Default|Gett))
  (bind _fan_rotator_01 (Variables|Default|GetFan%20Rotator_01))
  (bind _fan_rotator_02 (Variables|Default|GetFan%20Rotator_02))
  (bind _fan_rotator_03 (Variables|Default|GetFan%20Rotator_03))
  (bind _fan_rotator_04 (Variables|Default|GetFan%20Rotator_04))
  (bind _returnvalue (Math|Conversions|ToFloat(Integer) _t))
  (Variables|/Script/Engine.RotatingMovementComponent|SetRotationRate _fan_rotator_01 (Math|Rotator|MakeRotator 0.0 0.0 _returnvalue))
  (Components|Movement|SetUpdatedComponent _fan_rotator_01 (Variables|Default|GetPvot_Fan_01))
  (Variables|/Script/Engine.RotatingMovementComponent|SetRotationRate _fan_rotator_02 (Math|Rotator|MakeRotator 0.0 0.0 _returnvalue))
  (Components|Movement|SetUpdatedComponent _fan_rotator_02 (Variables|Default|GetPvot_Fan_02))
  (Variables|/Script/Engine.RotatingMovementComponent|SetRotationRate _fan_rotator_03 (Math|Rotator|MakeRotator 0.0 0.0 _returnvalue))
  (Components|Movement|SetUpdatedComponent _fan_rotator_03 (Variables|Default|GetPvot_Fan_03))
  (Variables|/Script/Engine.RotatingMovementComponent|SetRotationRate _fan_rotator_04 (Math|Rotator|MakeRotator 0.0 0.0 _returnvalue))
  (Components|Movement|SetUpdatedComponent _fan_rotator_04 (Variables|Default|GetPvot_Fan_04)))

(fn ConstructionScript
  (switch Utilities|FlowControl|Switch|SwitchonE_HeloRotorSpeeds (Variables|Default|GetFan%20RPM)
    (:NewEnumerator0
      (Variables|Default|Sett 0))
    (:NewEnumerator1
      (Variables|Default|Sett 200))
    (:NewEnumerator2
      (Variables|Default|Sett 800))))