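; BP_Air_Vent_2A is an air vent prop with a spinning fan.
; The construction script maps the FanRPM enum (off, low or high) to a rotation speed value.
; At BeginPlay that speed sets the roll rate of a rotating movement component, which is then bound to the fan mesh so only the fan turns.
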(event EventBeginPlay
  (bind _fan_rotator (Variables|Default|GetFan%20Rotator))
  (Variables|/Script/Engine.RotatingMovementComponent|SetRotationRate _fan_rotator (Math|Rotator|MakeRotator 0.0 0.0 (Math|Conversions|ToFloat(Integer) (Variables|Default|Gett))))
  (Components|Movement|SetUpdatedComponent _fan_rotator (Variables|Default|GetAir_Vent_2A_Fan)))

(fn ConstructionScript
  (switch Utilities|FlowControl|Switch|SwitchonE_HeloRotorSpeeds (Variables|Default|GetFan%20RPM)
    (:NewEnumerator0
      (Variables|Default|Sett 0))
    (:NewEnumerator1
      (Variables|Default|Sett 200))
    (:NewEnumerator2
      (Variables|Default|Sett 800))))