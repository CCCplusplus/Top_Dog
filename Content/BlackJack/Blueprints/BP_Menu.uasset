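; Blackjack menu actor that shows a Play button and hands off to the game.
; On BeginPlay it caches the BP_Logic game mode, then makes MenuRoot and its children visible.
; Clicking PlayButton calls StartGame on the logic, plays a continue sound and destroys the menu after a short delay.
; The touch handler is empty, and a leftover Play-and-delay sequence is disconnected.
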(event OnClicked(Playbutton)
  (params (TouchedComponent :type Primitive%20Component%20Object%20Reference) (ButtonPressed :type Key%20Structure))
  ;[1 1 1] Send menu to hidden possition
  (Default|StartGame (Variables|GameControl|GetLogic))
  ;;[1 1 1] Sound Continue
  (Audio|PlaySoundatLocation "/Game/BlackJack/Assets/Sounds/Frontend_Continue_Stereo_Cue.Frontend_Continue_Stereo_Cue" "0, 0, 0" "0, 0, 0" 1.0 1.0 0.0 0 0 0 0)
  (Utilities|FlowControl|Delay 0.7)
  (Actor|DestroyActor))

(event OnInputTouchBegin(Playbutton)
  (params (FingerIndex :type ETouchIndex%20Enum :default "Touch1") (TouchedComponent :type Primitive%20Component%20Object%20Reference))
  ;[1 1 1] Send menu to hidden possition
)

(event Custom|NewGame
  ;[1 1 1] Set initial menu position
  (Rendering|SetVisibility (Variables|BP_Menu|GetMenuRoot) true true))

(event EventBeginPlay
  ;[1 1 1] Initialise
  (bind _asbp_logic (Utilities|Casting|CastToBP_Logic (Game|GetGameMode)))
  (Variables|GameControl|SetLogic _asbp_logic)
  (CallFunction|NewGame))

(fn ConstructionScript)