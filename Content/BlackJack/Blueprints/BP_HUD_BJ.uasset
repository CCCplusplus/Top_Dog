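; Blackjack HUD that draws the player's cash, stakes, hand values and round result popups directly on the canvas.
; DrawHUD reads values from the BP_Logic game mode, scales text to screen height and projects hand totals from fixed world points, tinting totals over 21.
; UpdateHud maps an outcome index to two summary lines and a red or blue window, then hides it after a delay by calling itself.
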(event Custom|UpdateHud
  (params (Option :type Integer))
  ;[1 1 1] Display summary screen
  (Variables|Default|SetDisplayWindow true)
  (Variables|Default|SetOption (+ Option 1))
  (switch int (Variables|Default|GetOption)
    (:0
      (Variables|Default|SetDisplayWindow false)
      (Variables|Default|SetSummary%20Line%201 " ")
      (Variables|Default|SetSummary%20Line%202 " "))
    (:1
      (Variables|Default|SetSummary%20Line%201 "Over 21 points in cards")
      (Variables|Default|SetSummary%20Line%202 "YOU LOST")
      (Variables|Default|SetRed%20window true :!label _label)
      (Variables|Default|SetDisplayTime 2.0 :!label _label_2)
      (Utilities|FlowControl|Delay (Variables|Default|GetDisplayTime) :!label _label_3)
      (CallFunction|UpdateHud -1))
    (:2
      (Variables|Default|SetSummary%20Line%201 "Casino has the better hand")
      (Variables|Default|SetSummary%20Line%202 "YOU LOST")
      (goto _label))
    (:3
      (Variables|Default|SetSummary%20Line%201 "You have the better hand")
      (Variables|Default|SetSummary%20Line%202 "YOU WIN!")
      (Variables|Default|SetRed%20window false :!label _label_4)
      (goto _label_2))
    (:4
      (Variables|Default|SetSummary%20Line%201 "Even hands")
      (Variables|Default|SetSummary%20Line%202 "DRAW")
      (goto _label_4))
    (:5
      (Variables|Default|SetSummary%20Line%201 "Casino is over 21 points")
      (Variables|Default|SetSummary%20Line%202 "YOU WIN!")
      (goto _label_4))
    (:6
      (Variables|Default|SetSummary%20Line%201 "Out of cash!")
      (Variables|Default|SetSummary%20Line%202 "BANKRUPT")
      (Variables|Default|SetRed%20window true :!label _label_5)
      (Variables|Default|SetDisplayTime 3.0)
      (goto _label_3))
    (:7
      (Variables|Default|SetSummary%20Line%201 "Deck is almost empty")
      (Variables|Default|SetSummary%20Line%202 "GAME OVER")
      (goto _label_5))))

(event EventBeginPlay
  ;[1 1 1] Make Game Mode into a variable so we can retrieve information from it
  (bind _asbp_logic (Utilities|Casting|CastToBP_Logic (Game|GetGameMode)))
  (Variables|Default|SetGame%20mode%20BP _asbp_logic))

(event EventDrawHUD
  (params (SizeX :type Integer) (SizeY :type Integer))
  (bind _returnvalue (Class|HUD|Project "0,-300.000000, 0" true))
  (bind _returnvalue_2 (Class|HUD|Project "0,1250.000000, 0" true))
  (bind _game_mode_bp (Variables|Default|GetGame%20mode%20BP))
  (bind _game_mode_bp_2 (Variables|Default|GetGame%20mode%20BP))
  (bind _game_mode_bp_3 (Variables|Default|GetGame%20mode%20BP))
  (bind _summary_line_1 (Variables|Default|GetSummary%20Line%201))
  (bind _summary_line_2 (Variables|Default|GetSummary%20Line%202))
  (bind (_x _y) (Math|Vector|BreakVector _returnvalue))
  (bind (_x_2 _y_2) (Math|Vector|BreakVector _returnvalue_2))
  (bind _returnvalue_3 (Utilities|String|ToString(Name) _summary_line_1))
  (bind _returnvalue_4 (Utilities|String|ToString(Name) _summary_line_2))
  (bind _cashpool (Variables|/Game/BlackJack/Blueprints/BP_Logic.BP_Logic_C|GetCashPool _game_mode_bp))
  (bind _playershandvalue (Variables|/Game/BlackJack/Blueprints/BP_Logic.BP_Logic_C|GetPlayersHandValue _game_mode_bp_3))
  (bind _ai_hand_value (Variables|/Game/BlackJack/Blueprints/BP_Logic.BP_Logic_C|GetAI%20Hand%20Value _game_mode_bp_2))
  (bind _returnvalue_5 (Utilities|String|ToString(Integer) _ai_hand_value))
  (bind _returnvalue_6 (Utilities|String|ToString(Integer) _playershandvalue))
  (bind _returnvalue_7 (Math|Float|Round _cashpool))
  ;[1 1 1] Display HUD texts
  (Variables|Default|SetScreen%20width SizeX)
  (Variables|Default|SetScreen%20height SizeY)
  (if (Variables|Default|GetDisplayWindow)
    (Canvas|DrawTexture (select (Variables|Default|GetRed%20window) "/Game/BlackJack/Assets/Textures/T_MenuBackground_2.T_MenuBackground_2" "/Game/BlackJack/Assets/Textures/T_MenuBackground.T_MenuBackground") (- (* (Variables|Default|GetScreen%20width) 0.5) (* (/ (Math|Conversions|ToFloat(Integer) (Variables|Default|GetScreen%20height)) 1.4) 0.5)) (- (* (Variables|Default|GetScreen%20height) 0.5) (* (/ (/ (Math|Conversions|ToFloat(Integer) (Variables|Default|GetScreen%20height)) 1.4) 2.0) 0.5)) (/ (Math|Conversions|ToFloat(Integer) (Variables|Default|GetScreen%20height)) 1.4) (/ (/ (Math|Conversions|ToFloat(Integer) (Variables|Default|GetScreen%20height)) 1.4) 2.0) 0.0 0.0 1.0 1.0 "(R=1.000000,G=1.000000,B=1.000000,A=1.000000)"))
  (HUD|DrawText _returnvalue_3 "(R=1.000000,G=1.000000,B=1.000000,A=1.000000)" (- (* (Variables|Default|GetScreen%20width) 0.5) (* (.OutWidth (Class|HUD|GetTextSize _returnvalue_3 "/Engine/EngineFonts/RobotoDistanceField.RobotoDistanceField" (/ (Math|Conversions|ToFloat(Integer) (Variables|Default|GetScreen%20height)) 5e+02))) 0.5)) (- (* (Variables|Default|GetScreen%20height) 0.46) (* (.OutHeight (Class|HUD|GetTextSize _returnvalue_3 "/Engine/EngineFonts/RobotoDistanceField.RobotoDistanceField" (/ (Math|Conversions|ToFloat(Integer) (Variables|Default|GetScreen%20height)) 5e+02))) 0.5)) "/Engine/EngineFonts/RobotoDistanceField.RobotoDistanceField" (/ (Math|Conversions|ToFloat(Integer) (Variables|Default|GetScreen%20height)) 5e+02) false)
  (HUD|DrawText _returnvalue_4 "(R=1.000000,G=1.000000,B=1.000000,A=1.000000)" (- (* (Variables|Default|GetScreen%20width) 0.5) (* (.OutWidth (Class|HUD|GetTextSize _returnvalue_4 "/Engine/EngineFonts/RobotoDistanceField.RobotoDistanceField" (/ (Math|Conversions|ToFloat(Integer) (Variables|Default|GetScreen%20height)) 4e+02))) 0.5)) (- (* (Variables|Default|GetScreen%20height) 0.54) (* (.OutHeight (Class|HUD|GetTextSize _returnvalue_4 "/Engine/EngineFonts/RobotoDistanceField.RobotoDistanceField" (/ (Math|Conversions|ToFloat(Integer) (Variables|Default|GetScreen%20height)) 4e+02))) 0.5)) "/Engine/EngineFonts/RobotoDistanceField.RobotoDistanceField" (/ (Math|Conversions|ToFloat(Integer) (Variables|Default|GetScreen%20height)) 4e+02) false)
  ;[1 1 1] Display cash values
  (HUD|DrawText (Utilities|String|Append "Cash: " (Utilities|String|ToString(Integer) (Math|Float|Round (Variables|/Game/BlackJack/Blueprints/BP_Logic.BP_Logic_C|GetPlayersCash (Variables|Default|GetGame%20mode%20BP))))) "(R=1.000000,G=1.000000,B=1.000000,A=1.000000)" (/ (Math|Conversions|ToFloat(Integer) (Variables|Default|GetScreen%20width)) 3e+01) (/ (Math|Conversions|ToFloat(Integer) (Variables|Default|GetScreen%20height)) 16.0) "/Engine/EngineFonts/RobotoDistanceField.RobotoDistanceField" (/ (Math|Conversions|ToFloat(Integer) (Variables|Default|GetScreen%20height)) 5e+02) false) ; Draw player cash
  (if (> _returnvalue_7 0)
    (HUD|DrawText (Utilities|String|Append "Stakes: " (Utilities|String|ToString(Integer) _returnvalue_7)) "(R=1.000000,G=1.000000,B=1.000000,A=1.000000)" (/ (Math|Conversions|ToFloat(Integer) (Variables|Default|GetScreen%20width)) 3e+01) (/ (Math|Conversions|ToFloat(Integer) (Variables|Default|GetScreen%20height)) 8.5) "/Engine/EngineFonts/RobotoDistanceField.RobotoDistanceField" (/ (Math|Conversions|ToFloat(Integer) (Variables|Default|GetScreen%20height)) 5e+02) false) ; Draw player stakes
  )
  ;[1 1 1] Display hand values
  (if (Variables|/Game/BlackJack/Blueprints/BP_Logic.BP_Logic_C|GetShow%20player%20hand%20value (Variables|Default|GetGame%20mode%20BP))
    (HUD|DrawText _returnvalue_6 (Math|Color|SelectColor "(R=1.000000,G=0.300000,B=0.100000,A=1.000000)" "(R=1.000000,G=1.000000,B=1.000000,A=1.000000)" (> _playershandvalue 21)) (- _x_2 (* (.OutWidth (Class|HUD|GetTextSize _returnvalue_6 "/Engine/EngineFonts/RobotoDistanceField.RobotoDistanceField" (/ (Math|Conversions|ToFloat(Integer) (Variables|Default|GetScreen%20height)) 3e+02))) 0.5)) _y_2 "/Engine/EngineFonts/RobotoDistanceField.RobotoDistanceField" (/ (Math|Conversions|ToFloat(Integer) (Variables|Default|GetScreen%20height)) 3e+02) false) ; Draw player hand value
    (if (Variables|/Game/BlackJack/Blueprints/BP_Logic.BP_Logic_C|GetShow%20AI%20hand%20value (Variables|Default|GetGame%20mode%20BP))
      (HUD|DrawText _returnvalue_5 (Math|Color|SelectColor "(R=1.000000,G=0.300000,B=0.100000,A=1.000000)" "(R=1.000000,G=1.000000,B=1.000000,A=1.000000)" (> _ai_hand_value 21)) (- _x (* (.OutWidth (Class|HUD|GetTextSize _returnvalue_5 "/Engine/EngineFonts/RobotoDistanceField.RobotoDistanceField" (/ (Math|Conversions|ToFloat(Integer) (Variables|Default|GetScreen%20height)) 4e+02))) 0.5)) _y "/Engine/EngineFonts/RobotoDistanceField.RobotoDistanceField" (/ (Math|Conversions|ToFloat(Integer) (Variables|Default|GetScreen%20height)) 4e+02) false) ; Draw AI hand value
    )))

(fn ConstructionScript
  ;[1 1 1] Setup initial HUD state
  (Variables|Default|SetOption 0)
  (Variables|Default|SetDisplayTime 5.0)
  (Variables|Default|SetDisplayWindow false)
  (CallFunction|UpdateHud -1))