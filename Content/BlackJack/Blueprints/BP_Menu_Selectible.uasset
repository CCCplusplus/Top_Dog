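; Blackjack menu actor with four 3D chip buttons that choose an option of 1, 3, 5 or 7, apparently deck count.
; Click or touch resets all chips, highlights one, passes the value to BP_Logic.InitialSetup, plays a sound and destroys the actor.
; The construction script caches chip locations and material, then calls PressedOnStart for button three through that same path, before BeginPlay sets Logic.
; Chip-raising nodes are disconnected.
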(event OnInputTouchBegin(Button3)
  (params (FingerIndex :type ETouchIndex%20Enum :default "Touch1") (TouchedComponent :type Primitive%20Component%20Object%20Reference))
  (bind _button1 (Variables|BP_Menu_Selectible|GetButton1))
  (bind _button4 (Variables|BP_Menu_Selectible|GetButton4))
  (bind _button3 (Variables|BP_Menu_Selectible|GetButton3))
  (bind _initialmaterial (Variables|Default|GetInitialMaterial))
  (bind _button2 (Variables|BP_Menu_Selectible|GetButton2))
  ;[1 1 1] Click buttons
  (Utilities|FlowControl|Sequence
    (:then_0
      ;[1 1 1] Unclick buttons
      (Utilities|FlowControl|Sequence
        (:then_0
          (Transformation|SetRelativeLocation _button1 (Variables|Default|GetButton1Location) false false)
          (Rendering|Material|SetMaterial _button1 0 _initialmaterial))
        (:then_1
          (Transformation|SetRelativeLocation _button2 (Variables|Default|GetButton2Location) false false)
          (Rendering|Material|SetMaterial _button2 0 _initialmaterial))
        (:then_2
          (Transformation|SetRelativeLocation _button3 (Variables|Default|GetButton3Location) false false)
          (Rendering|Material|SetMaterial _button3 0 _initialmaterial))
        (:then_3
          (Transformation|SetRelativeLocation _button4 (Variables|Default|GetButton4Location) false false)
          (Rendering|Material|SetMaterial _button4 0 _initialmaterial))))
    (:then_1
      (Rendering|Material|SetMaterial (Variables|BP_Menu_Selectible|GetButton3) 0 "/Game/BlackJack/Assets/Materials/M_CasinoChip_01_E_Inst.M_CasinoChip_01_E_Inst")
      ;[1 1 1] Sending Output
      (Variables|Default|SetOutput%20-%20SelectedOption 5)
      (Default|InitialSetup (Variables|GameControl|GetLogic) (Variables|Default|GetOutput%20-%20SelectedOption))
      ;;[1 1 1] Sound Deck Number Pressed
      (Audio|PlaySoundatLocation "/Game/BlackJack/Assets/Sounds/Frontend_ChipSelect_Stereo_Cue.Frontend_ChipSelect_Stereo_Cue" "0, 0, 0" "0, 0, 0" 1.0 1.0 0.0 0 0 0 0)
      (Actor|DestroyActor))))

(event OnInputTouchBegin(Button4)
  (params (FingerIndex :type ETouchIndex%20Enum :default "Touch1") (TouchedComponent :type Primitive%20Component%20Object%20Reference))
  (bind _button1 (Variables|BP_Menu_Selectible|GetButton1))
  (bind _button4 (Variables|BP_Menu_Selectible|GetButton4))
  (bind _button3 (Variables|BP_Menu_Selectible|GetButton3))
  (bind _initialmaterial (Variables|Default|GetInitialMaterial))
  (bind _button2 (Variables|BP_Menu_Selectible|GetButton2))
  ;[1 1 1] Click buttons
  (Utilities|FlowControl|Sequence
    (:then_0
      ;[1 1 1] Unclick buttons
      (Utilities|FlowControl|Sequence
        (:then_0
          (Transformation|SetRelativeLocation _button1 (Variables|Default|GetButton1Location) false false)
          (Rendering|Material|SetMaterial _button1 0 _initialmaterial))
        (:then_1
          (Transformation|SetRelativeLocation _button2 (Variables|Default|GetButton2Location) false false)
          (Rendering|Material|SetMaterial _button2 0 _initialmaterial))
        (:then_2
          (Transformation|SetRelativeLocation _button3 (Variables|Default|GetButton3Location) false false)
          (Rendering|Material|SetMaterial _button3 0 _initialmaterial))
        (:then_3
          (Transformation|SetRelativeLocation _button4 (Variables|Default|GetButton4Location) false false)
          (Rendering|Material|SetMaterial _button4 0 _initialmaterial))))
    (:then_1
      (Rendering|Material|SetMaterial (Variables|BP_Menu_Selectible|GetButton4) 0 "/Game/BlackJack/Assets/Materials/M_CasinoChip_01_E_Inst.M_CasinoChip_01_E_Inst")
      ;[1 1 1] Sending Output
      (Variables|Default|SetOutput%20-%20SelectedOption 7)
      (Default|InitialSetup (Variables|GameControl|GetLogic) (Variables|Default|GetOutput%20-%20SelectedOption))
      ;;[1 1 1] Sound Deck Number Pressed
      (Audio|PlaySoundatLocation "/Game/BlackJack/Assets/Sounds/Frontend_ChipSelect_Stereo_Cue.Frontend_ChipSelect_Stereo_Cue" "0, 0, 0" "0, 0, 0" 1.0 1.0 0.0 0 0 0 0)
      (Actor|DestroyActor))))

(event OnClicked(Button1)
  (params (TouchedComponent :type Primitive%20Component%20Object%20Reference) (ButtonPressed :type Key%20Structure :default "None"))
  (bind _button1 (Variables|BP_Menu_Selectible|GetButton1))
  (bind _button4 (Variables|BP_Menu_Selectible|GetButton4))
  (bind _button3 (Variables|BP_Menu_Selectible|GetButton3))
  (bind _initialmaterial (Variables|Default|GetInitialMaterial))
  (bind _button2 (Variables|BP_Menu_Selectible|GetButton2))
  ;[1 1 1] Click buttons
  (Utilities|FlowControl|Sequence
    (:then_0
      ;[1 1 1] Unclick buttons
      (Utilities|FlowControl|Sequence
        (:then_0
          (Transformation|SetRelativeLocation _button1 (Variables|Default|GetButton1Location) false false)
          (Rendering|Material|SetMaterial _button1 0 _initialmaterial))
        (:then_1
          (Transformation|SetRelativeLocation _button2 (Variables|Default|GetButton2Location) false false)
          (Rendering|Material|SetMaterial _button2 0 _initialmaterial))
        (:then_2
          (Transformation|SetRelativeLocation _button3 (Variables|Default|GetButton3Location) false false)
          (Rendering|Material|SetMaterial _button3 0 _initialmaterial))
        (:then_3
          (Transformation|SetRelativeLocation _button4 (Variables|Default|GetButton4Location) false false)
          (Rendering|Material|SetMaterial _button4 0 _initialmaterial))))
    (:then_1
      (Rendering|Material|SetMaterial (Variables|BP_Menu_Selectible|GetButton1) 0 "/Game/BlackJack/Assets/Materials/M_CasinoChip_01_E_Inst.M_CasinoChip_01_E_Inst")
      ;[1 1 1] Sending Output
      (Variables|Default|SetOutput%20-%20SelectedOption 1)
      (Default|InitialSetup (Variables|GameControl|GetLogic) (Variables|Default|GetOutput%20-%20SelectedOption))
      ;;[1 1 1] Sound Deck Number Pressed
      (Audio|PlaySoundatLocation "/Game/BlackJack/Assets/Sounds/Frontend_ChipSelect_Stereo_Cue.Frontend_ChipSelect_Stereo_Cue" "0, 0, 0" "0, 0, 0" 1.0 1.0 0.0 0 0 0 0)
      (Actor|DestroyActor))))

(event OnClicked(Button2)
  (params (TouchedComponent :type Primitive%20Component%20Object%20Reference) (ButtonPressed :type Key%20Structure :default "None"))
  (bind _button1 (Variables|BP_Menu_Selectible|GetButton1))
  (bind _button4 (Variables|BP_Menu_Selectible|GetButton4))
  (bind _button3 (Variables|BP_Menu_Selectible|GetButton3))
  (bind _initialmaterial (Variables|Default|GetInitialMaterial))
  (bind _button2 (Variables|BP_Menu_Selectible|GetButton2))
  ;[1 1 1] Click buttons
  (Utilities|FlowControl|Sequence
    (:then_0
      ;[1 1 1] Unclick buttons
      (Utilities|FlowControl|Sequence
        (:then_0
          (Transformation|SetRelativeLocation _button1 (Variables|Default|GetButton1Location) false false)
          (Rendering|Material|SetMaterial _button1 0 _initialmaterial))
        (:then_1
          (Transformation|SetRelativeLocation _button2 (Variables|Default|GetButton2Location) false false)
          (Rendering|Material|SetMaterial _button2 0 _initialmaterial))
        (:then_2
          (Transformation|SetRelativeLocation _button3 (Variables|Default|GetButton3Location) false false)
          (Rendering|Material|SetMaterial _button3 0 _initialmaterial))
        (:then_3
          (Transformation|SetRelativeLocation _button4 (Variables|Default|GetButton4Location) false false)
          (Rendering|Material|SetMaterial _button4 0 _initialmaterial))))
    (:then_1
      (Rendering|Material|SetMaterial (Variables|BP_Menu_Selectible|GetButton2) 0 "/Game/BlackJack/Assets/Materials/M_CasinoChip_01_E_Inst.M_CasinoChip_01_E_Inst")
      ;[1 1 1] Sending Output
      (Variables|Default|SetOutput%20-%20SelectedOption 3)
      (Default|InitialSetup (Variables|GameControl|GetLogic) (Variables|Default|GetOutput%20-%20SelectedOption))
      ;;[1 1 1] Sound Deck Number Pressed
      (Audio|PlaySoundatLocation "/Game/BlackJack/Assets/Sounds/Frontend_ChipSelect_Stereo_Cue.Frontend_ChipSelect_Stereo_Cue" "0, 0, 0" "0, 0, 0" 1.0 1.0 0.0 0 0 0 0)
      (Actor|DestroyActor))))

(event OnClicked(Button3)
  (params (TouchedComponent :type Primitive%20Component%20Object%20Reference) (ButtonPressed :type Key%20Structure :default "None"))
  (bind _button1 (Variables|BP_Menu_Selectible|GetButton1))
  (bind _button4 (Variables|BP_Menu_Selectible|GetButton4))
  (bind _button3 (Variables|BP_Menu_Selectible|GetButton3))
  (bind _initialmaterial (Variables|Default|GetInitialMaterial))
  (bind _button2 (Variables|BP_Menu_Selectible|GetButton2))
  ;[1 1 1] Click buttons
  (Utilities|FlowControl|Sequence
    (:then_0
      ;[1 1 1] Unclick buttons
      (Utilities|FlowControl|Sequence
        (:then_0
          (Transformation|SetRelativeLocation _button1 (Variables|Default|GetButton1Location) false false)
          (Rendering|Material|SetMaterial _button1 0 _initialmaterial))
        (:then_1
          (Transformation|SetRelativeLocation _button2 (Variables|Default|GetButton2Location) false false)
          (Rendering|Material|SetMaterial _button2 0 _initialmaterial))
        (:then_2
          (Transformation|SetRelativeLocation _button3 (Variables|Default|GetButton3Location) false false)
          (Rendering|Material|SetMaterial _button3 0 _initialmaterial))
        (:then_3
          (Transformation|SetRelativeLocation _button4 (Variables|Default|GetButton4Location) false false)
          (Rendering|Material|SetMaterial _button4 0 _initialmaterial))))
    (:then_1
      (Rendering|Material|SetMaterial (Variables|BP_Menu_Selectible|GetButton3) 0 "/Game/BlackJack/Assets/Materials/M_CasinoChip_01_E_Inst.M_CasinoChip_01_E_Inst")
      ;[1 1 1] Sending Output
      (Variables|Default|SetOutput%20-%20SelectedOption 5)
      (Default|InitialSetup (Variables|GameControl|GetLogic) (Variables|Default|GetOutput%20-%20SelectedOption))
      ;;[1 1 1] Sound Deck Number Pressed
      (Audio|PlaySoundatLocation "/Game/BlackJack/Assets/Sounds/Frontend_ChipSelect_Stereo_Cue.Frontend_ChipSelect_Stereo_Cue" "0, 0, 0" "0, 0, 0" 1.0 1.0 0.0 0 0 0 0)
      (Actor|DestroyActor))))

(event OnInputTouchBegin(Button1)
  (params (FingerIndex :type ETouchIndex%20Enum :default "Touch1") (TouchedComponent :type Primitive%20Component%20Object%20Reference))
  (bind _button1 (Variables|BP_Menu_Selectible|GetButton1))
  (bind _button4 (Variables|BP_Menu_Selectible|GetButton4))
  (bind _button3 (Variables|BP_Menu_Selectible|GetButton3))
  (bind _initialmaterial (Variables|Default|GetInitialMaterial))
  (bind _button2 (Variables|BP_Menu_Selectible|GetButton2))
  ;[1 1 1] Click buttons
  (Utilities|FlowControl|Sequence
    (:then_0
      ;[1 1 1] Unclick buttons
      (Utilities|FlowControl|Sequence
        (:then_0
          (Transformation|SetRelativeLocation _button1 (Variables|Default|GetButton1Location) false false)
          (Rendering|Material|SetMaterial _button1 0 _initialmaterial))
        (:then_1
          (Transformation|SetRelativeLocation _button2 (Variables|Default|GetButton2Location) false false)
          (Rendering|Material|SetMaterial _button2 0 _initialmaterial))
        (:then_2
          (Transformation|SetRelativeLocation _button3 (Variables|Default|GetButton3Location) false false)
          (Rendering|Material|SetMaterial _button3 0 _initialmaterial))
        (:then_3
          (Transformation|SetRelativeLocation _button4 (Variables|Default|GetButton4Location) false false)
          (Rendering|Material|SetMaterial _button4 0 _initialmaterial))))
    (:then_1
      (Rendering|Material|SetMaterial (Variables|BP_Menu_Selectible|GetButton1) 0 "/Game/BlackJack/Assets/Materials/M_CasinoChip_01_E_Inst.M_CasinoChip_01_E_Inst")
      ;[1 1 1] Sending Output
      (Variables|Default|SetOutput%20-%20SelectedOption 1)
      (Default|InitialSetup (Variables|GameControl|GetLogic) (Variables|Default|GetOutput%20-%20SelectedOption))
      ;;[1 1 1] Sound Deck Number Pressed
      (Audio|PlaySoundatLocation "/Game/BlackJack/Assets/Sounds/Frontend_ChipSelect_Stereo_Cue.Frontend_ChipSelect_Stereo_Cue" "0, 0, 0" "0, 0, 0" 1.0 1.0 0.0 0 0 0 0)
      (Actor|DestroyActor))))

(event OnClicked(Button4)
  (params (TouchedComponent :type Primitive%20Component%20Object%20Reference) (ButtonPressed :type Key%20Structure :default "None"))
  (bind _button1 (Variables|BP_Menu_Selectible|GetButton1))
  (bind _button4 (Variables|BP_Menu_Selectible|GetButton4))
  (bind _button3 (Variables|BP_Menu_Selectible|GetButton3))
  (bind _initialmaterial (Variables|Default|GetInitialMaterial))
  (bind _button2 (Variables|BP_Menu_Selectible|GetButton2))
  ;[1 1 1] Click buttons
  (Utilities|FlowControl|Sequence
    (:then_0
      ;[1 1 1] Unclick buttons
      (Utilities|FlowControl|Sequence
        (:then_0
          (Transformation|SetRelativeLocation _button1 (Variables|Default|GetButton1Location) false false)
          (Rendering|Material|SetMaterial _button1 0 _initialmaterial))
        (:then_1
          (Transformation|SetRelativeLocation _button2 (Variables|Default|GetButton2Location) false false)
          (Rendering|Material|SetMaterial _button2 0 _initialmaterial))
        (:then_2
          (Transformation|SetRelativeLocation _button3 (Variables|Default|GetButton3Location) false false)
          (Rendering|Material|SetMaterial _button3 0 _initialmaterial))
        (:then_3
          (Transformation|SetRelativeLocation _button4 (Variables|Default|GetButton4Location) false false)
          (Rendering|Material|SetMaterial _button4 0 _initialmaterial))))
    (:then_1
      (Rendering|Material|SetMaterial (Variables|BP_Menu_Selectible|GetButton4) 0 "/Game/BlackJack/Assets/Materials/M_CasinoChip_01_E_Inst.M_CasinoChip_01_E_Inst")
      ;[1 1 1] Sending Output
      (Variables|Default|SetOutput%20-%20SelectedOption 7)
      (Default|InitialSetup (Variables|GameControl|GetLogic) (Variables|Default|GetOutput%20-%20SelectedOption))
      ;;[1 1 1] Sound Deck Number Pressed
      (Audio|PlaySoundatLocation "/Game/BlackJack/Assets/Sounds/Frontend_ChipSelect_Stereo_Cue.Frontend_ChipSelect_Stereo_Cue" "0, 0, 0" "0, 0, 0" 1.0 1.0 0.0 0 0 0 0)
      (Actor|DestroyActor))))

(event OnInputTouchBegin(Button2)
  (params (FingerIndex :type ETouchIndex%20Enum :default "Touch1") (TouchedComponent :type Primitive%20Component%20Object%20Reference))
  (bind _button1 (Variables|BP_Menu_Selectible|GetButton1))
  (bind _button4 (Variables|BP_Menu_Selectible|GetButton4))
  (bind _button3 (Variables|BP_Menu_Selectible|GetButton3))
  (bind _initialmaterial (Variables|Default|GetInitialMaterial))
  (bind _button2 (Variables|BP_Menu_Selectible|GetButton2))
  ;[1 1 1] Click buttons
  (Utilities|FlowControl|Sequence
    (:then_0
      ;[1 1 1] Unclick buttons
      (Utilities|FlowControl|Sequence
        (:then_0
          (Transformation|SetRelativeLocation _button1 (Variables|Default|GetButton1Location) false false)
          (Rendering|Material|SetMaterial _button1 0 _initialmaterial))
        (:then_1
          (Transformation|SetRelativeLocation _button2 (Variables|Default|GetButton2Location) false false)
          (Rendering|Material|SetMaterial _button2 0 _initialmaterial))
        (:then_2
          (Transformation|SetRelativeLocation _button3 (Variables|Default|GetButton3Location) false false)
          (Rendering|Material|SetMaterial _button3 0 _initialmaterial))
        (:then_3
          (Transformation|SetRelativeLocation _button4 (Variables|Default|GetButton4Location) false false)
          (Rendering|Material|SetMaterial _button4 0 _initialmaterial))))
    (:then_1
      (Rendering|Material|SetMaterial (Variables|BP_Menu_Selectible|GetButton2) 0 "/Game/BlackJack/Assets/Materials/M_CasinoChip_01_E_Inst.M_CasinoChip_01_E_Inst")
      ;[1 1 1] Sending Output
      (Variables|Default|SetOutput%20-%20SelectedOption 3)
      (Default|InitialSetup (Variables|GameControl|GetLogic) (Variables|Default|GetOutput%20-%20SelectedOption))
      ;;[1 1 1] Sound Deck Number Pressed
      (Audio|PlaySoundatLocation "/Game/BlackJack/Assets/Sounds/Frontend_ChipSelect_Stereo_Cue.Frontend_ChipSelect_Stereo_Cue" "0, 0, 0" "0, 0, 0" 1.0 1.0 0.0 0 0 0 0)
      (Actor|DestroyActor))))

(event Custom|PressedOnStart
  (bind _button1 (Variables|BP_Menu_Selectible|GetButton1))
  (bind _button4 (Variables|BP_Menu_Selectible|GetButton4))
  (bind _button3 (Variables|BP_Menu_Selectible|GetButton3))
  (bind _initialmaterial (Variables|Default|GetInitialMaterial))
  (bind _button2 (Variables|BP_Menu_Selectible|GetButton2))
  ;[1 1 1] Pressed on start
  (switch int (Variables|Default|GetDefaultPressedButton)
    (:1
      ;[1 1 1] Click buttons
      (Utilities|FlowControl|Sequence
        (:then_0
          ;[1 1 1] Unclick buttons
          (Utilities|FlowControl|Sequence :!label _label
            (:then_0
              (Transformation|SetRelativeLocation _button1 (Variables|Default|GetButton1Location) false false)
              (Rendering|Material|SetMaterial _button1 0 _initialmaterial))
            (:then_1
              (Transformation|SetRelativeLocation _button2 (Variables|Default|GetButton2Location) false false)
              (Rendering|Material|SetMaterial _button2 0 _initialmaterial))
            (:then_2
              (Transformation|SetRelativeLocation _button3 (Variables|Default|GetButton3Location) false false)
              (Rendering|Material|SetMaterial _button3 0 _initialmaterial))
            (:then_3
              (Transformation|SetRelativeLocation _button4 (Variables|Default|GetButton4Location) false false)
              (Rendering|Material|SetMaterial _button4 0 _initialmaterial))))
        (:then_1
          (Rendering|Material|SetMaterial (Variables|BP_Menu_Selectible|GetButton1) 0 "/Game/BlackJack/Assets/Materials/M_CasinoChip_01_E_Inst.M_CasinoChip_01_E_Inst")
          ;[1 1 1] Sending Output
          (Variables|Default|SetOutput%20-%20SelectedOption 1)
          (Default|InitialSetup (Variables|GameControl|GetLogic) (Variables|Default|GetOutput%20-%20SelectedOption) :!label _label_2)
          ;;[1 1 1] Sound Deck Number Pressed
          (Audio|PlaySoundatLocation "/Game/BlackJack/Assets/Sounds/Frontend_ChipSelect_Stereo_Cue.Frontend_ChipSelect_Stereo_Cue" "0, 0, 0" "0, 0, 0" 1.0 1.0 0.0 0 0 0 0)
          (Actor|DestroyActor))))
    (:2
      (Utilities|FlowControl|Sequence
        (:then_0
          (goto _label))
        (:then_1
          (Rendering|Material|SetMaterial (Variables|BP_Menu_Selectible|GetButton2) 0 "/Game/BlackJack/Assets/Materials/M_CasinoChip_01_E_Inst.M_CasinoChip_01_E_Inst")
          (Variables|Default|SetOutput%20-%20SelectedOption 3)
          (goto _label_2))))
    (:3
      (Utilities|FlowControl|Sequence
        (:then_0
          (goto _label))
        (:then_1
          (Rendering|Material|SetMaterial (Variables|BP_Menu_Selectible|GetButton3) 0 "/Game/BlackJack/Assets/Materials/M_CasinoChip_01_E_Inst.M_CasinoChip_01_E_Inst")
          (Variables|Default|SetOutput%20-%20SelectedOption 5)
          (goto _label_2))))
    (:4
      (Utilities|FlowControl|Sequence
        (:then_0
          (goto _label))
        (:then_1
          (Rendering|Material|SetMaterial (Variables|BP_Menu_Selectible|GetButton4) 0 "/Game/BlackJack/Assets/Materials/M_CasinoChip_01_E_Inst.M_CasinoChip_01_E_Inst")
          (Variables|Default|SetOutput%20-%20SelectedOption 7)
          (goto _label_2))))))

(event EventBeginPlay
  ;[1 1 1] Initialise
  (bind _asbp_logic (Utilities|Casting|CastToBP_Logic (Game|GetGameMode)))
  (Variables|GameControl|SetLogic _asbp_logic))

(fn ConstructionScript
  (bind _button4 (Variables|BP_Menu_Selectible|GetButton4))
  ;[1 1 1] Setup Initial variables
  (Variables|Default|SetButton1Location (Variables|/Script/Engine.SceneComponent|GetRelativeLocation (Variables|BP_Menu_Selectible|GetButton1)))
  (Variables|Default|SetButton2Location (Variables|/Script/Engine.SceneComponent|GetRelativeLocation (Variables|BP_Menu_Selectible|GetButton2)))
  (Variables|Default|SetButton3Location (Variables|/Script/Engine.SceneComponent|GetRelativeLocation (Variables|BP_Menu_Selectible|GetButton3)))
  (Variables|Default|SetButton4Location (Variables|/Script/Engine.SceneComponent|GetRelativeLocation _button4))
  (Variables|Default|SetInitialMaterial (Rendering|Material|GetMaterial _button4 0))
  ;[1 1 1] Pressed on start
  (Variables|Default|SetDefaultPressedButton 3)
  (CallFunction|PressedonStart))