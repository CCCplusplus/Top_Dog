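; BP_Sound plays randomized, layered casino background ambience for the Blackjack game, starting on BeginPlay.
; Two channels each alternate between two audio components via FlipFlop, picking one of four casino loop cues at random.
; Timelines drive each component's volume, and their Start New Loop events trigger the next component through a Gate, chaining playback continuously.
; Channel 2 adds a random delay and pitch variation and uses a wider volume range.
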(event EventBeginPlay
  (bind _soundcasinoambience01 (Variables|BP_Sound|GetSoundCasinoAmbience01))
  (bind _soundcasinoambience02 (Variables|BP_Sound|GetSoundCasinoAmbience02))
  (bind _soundcasinoambience03 (Variables|BP_Sound|GetSoundCasinoAmbience03))
  (bind _soundcasinoambience04 (Variables|BP_Sound|GetSoundCasinoAmbience04))
  (Utilities|FlowControl|Sequence
    (:then_0
      ;[1 1 1] Channel 1
      (Utilities|FlowControl|FlipFlop :!label _label
        (:A
          (switch int (Math|Random|RandomIntegerinRange 0 3)
            (:0
              (Audio|Components|Audio|SetSound _soundcasinoambience04 "/Game/BlackJack/Assets/Sounds/AmbientCasino01_Loop_Stereo_Cue.AmbientCasino01_Loop_Stereo_Cue"))
            (:1
              (Audio|Components|Audio|SetSound _soundcasinoambience04 "/Game/BlackJack/Assets/Sounds/AmbientCasino02_Loop_Stereo_Cue.AmbientCasino02_Loop_Stereo_Cue"))
            (:2
              (Audio|Components|Audio|SetSound _soundcasinoambience04 "/Game/BlackJack/Assets/Sounds/AmbientCasino03_Loop_Stereo_Cue.AmbientCasino03_Loop_Stereo_Cue"))
            (:3
              (Audio|Components|Audio|SetSound _soundcasinoambience04 "/Game/BlackJack/Assets/Sounds/AmbientCasino04_Loop_Stereo_Cue.AmbientCasino04_Loop_Stereo_Cue")))
          (Audio|Components|Audio|Play _soundcasinoambience04 0.0)
          (bind _volume (Timeline|Timeline_3 PlayFromStart)
            (:Update
              (Audio|Components|Audio|SetVolumeMultiplier (Variables|BP_Sound|GetSoundCasinoAmbience04) (Math|Float|Lerp 0.2 0.5 _volume) :!class /Script/Engine.AudioComponent))
            (:StartNewLoop
              (Utilities|FlowControl|Gate false :!label _label_2
                (:Exit
                  (goto _label))))))
        (:B
          (switch int (Math|Random|RandomIntegerinRange 0 3)
            (:0
              (Audio|Components|Audio|SetSound _soundcasinoambience03 "/Game/BlackJack/Assets/Sounds/AmbientCasino01_Loop_Stereo_Cue.AmbientCasino01_Loop_Stereo_Cue"))
            (:1
              (Audio|Components|Audio|SetSound _soundcasinoambience03 "/Game/BlackJack/Assets/Sounds/AmbientCasino02_Loop_Stereo_Cue.AmbientCasino02_Loop_Stereo_Cue"))
            (:2
              (Audio|Components|Audio|SetSound _soundcasinoambience03 "/Game/BlackJack/Assets/Sounds/AmbientCasino03_Loop_Stereo_Cue.AmbientCasino03_Loop_Stereo_Cue"))
            (:3
              (Audio|Components|Audio|SetSound _soundcasinoambience03 "/Game/BlackJack/Assets/Sounds/AmbientCasino04_Loop_Stereo_Cue.AmbientCasino04_Loop_Stereo_Cue")))
          (Audio|Components|Audio|Play _soundcasinoambience03 0.0)
          (bind _volume_2 (Timeline|Timeline_4 PlayFromStart)
            (:Update
              (Audio|Components|Audio|SetVolumeMultiplier (Variables|BP_Sound|GetSoundCasinoAmbience03) (Math|Float|Lerp 0.2 0.5 _volume_2) :!class /Script/Engine.AudioComponent))
            (:StartNewLoop
              (goto _label_2))))))
    (:then_1
      ;[1 1 1] Channel 2
      (Utilities|FlowControl|Delay (Math|Random|RandomFloatinRange 1.0 4.0) :!label _label_3)
      (Audio|Components|Audio|SetPitchMultiplier (Variables|BP_Sound|GetSoundCasinoAmbience01) (Math|Random|RandomFloatinRange 0.9 1.1))
      (Utilities|FlowControl|FlipFlop
        (:A
          (switch int (Math|Random|RandomIntegerinRange 0 3)
            (:0
              (Audio|Components|Audio|SetSound _soundcasinoambience01 "/Game/BlackJack/Assets/Sounds/AmbientCasino01_Loop_Stereo_Cue.AmbientCasino01_Loop_Stereo_Cue"))
            (:1
              (Audio|Components|Audio|SetSound _soundcasinoambience01 "/Game/BlackJack/Assets/Sounds/AmbientCasino02_Loop_Stereo_Cue.AmbientCasino02_Loop_Stereo_Cue"))
            (:2
              (Audio|Components|Audio|SetSound _soundcasinoambience01 "/Game/BlackJack/Assets/Sounds/AmbientCasino03_Loop_Stereo_Cue.AmbientCasino03_Loop_Stereo_Cue"))
            (:3
              (Audio|Components|Audio|SetSound _soundcasinoambience01 "/Game/BlackJack/Assets/Sounds/AmbientCasino04_Loop_Stereo_Cue.AmbientCasino04_Loop_Stereo_Cue")))
          (Audio|Components|Audio|Play _soundcasinoambience01 0.0)
          (bind _volume_3 (Timeline|Timeline_2 PlayFromStart)
            (:Update
              (Audio|Components|Audio|SetVolumeMultiplier (Variables|BP_Sound|GetSoundCasinoAmbience01) (Math|Float|Lerp 0.0 1.0 _volume_3) :!class /Script/Engine.AudioComponent))
            (:StartNewLoop
              (Utilities|FlowControl|Gate false :!label _label_4
                (:Exit
                  (goto _label_3))))))
        (:B
          (switch int (Math|Random|RandomIntegerinRange 0 3)
            (:0
              (Audio|Components|Audio|SetSound _soundcasinoambience02 "/Game/BlackJack/Assets/Sounds/AmbientCasino01_Loop_Stereo_Cue.AmbientCasino01_Loop_Stereo_Cue"))
            (:1
              (Audio|Components|Audio|SetSound _soundcasinoambience02 "/Game/BlackJack/Assets/Sounds/AmbientCasino02_Loop_Stereo_Cue.AmbientCasino02_Loop_Stereo_Cue"))
            (:2
              (Audio|Components|Audio|SetSound _soundcasinoambience02 "/Game/BlackJack/Assets/Sounds/AmbientCasino03_Loop_Stereo_Cue.AmbientCasino03_Loop_Stereo_Cue"))
            (:3
              (Audio|Components|Audio|SetSound _soundcasinoambience02 "/Game/BlackJack/Assets/Sounds/AmbientCasino04_Loop_Stereo_Cue.AmbientCasino04_Loop_Stereo_Cue")))
          (Audio|Components|Audio|Play _soundcasinoambience02 0.0)
          (bind _volume_4 (Timeline|Timeline_0 PlayFromStart)
            (:Update
              (Audio|Components|Audio|SetVolumeMultiplier (Variables|BP_Sound|GetSoundCasinoAmbience02) (Math|Float|Lerp 0.0 1.0 _volume_4) :!class /Script/Engine.AudioComponent))
            (:StartNewLoop
              (goto _label_4))))))))

(fn ConstructionScript)