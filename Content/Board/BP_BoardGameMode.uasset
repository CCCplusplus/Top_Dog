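; Game mode for a party board game that alternates rounds of character die-roll turns with random minigames and finishes with an endgame dialog cutscene.
; Turns chain through each character's OnTurnEnded event; an empty round queue decrements the round count and opens a minigame level.
; Board state persists across level loads in a PartySave slot.
; Game instance flags steer resumption after minigames or gambles and identify the winner to pay.
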(event Custom|InitiateRound
  (Variables|Default|SetroundOrder (Variables|Default|GetturnOrder))
  (CallFunction|StartTurn))

(event Custom|NextTurn
  (Utilities|Array|RemoveIndex (Variables|Default|GetroundOrder))
  (bind _asbp_board_game_instance (Utilities|Casting|CastToBP_BoardGameInstance (Game|GetGameInstance)))
  (if (Utilities|Array|IsEmpty (Variables|Default|GetroundOrder))
    (if (not (Variables|/Game/Board/BP_BoardGameInstance.BP_BoardGameInstance_C|GetfromGamble _asbp_board_game_instance))
      (CallFunction|EndRound))
    (else
      (CallFunction|StartTurn))))

(event Custom|StartTurn
  (bind _roundorder (Variables|Default|GetroundOrder))
  (bind _output (Utilities|Array|Get(acopy) _roundorder))
  (Utilities|FlowControl|Delay 0.2)
  (Default|RollDie _output)
  (EventDispatchers|BindEventtoOnTurnEnded _output (delegate Custom|NextTurn)))

(event Custom|EndRound
  (Math|Integer|DecrementInt (Variables|Default|Getrounds)
    (:%20%20
      (CallFunction|SaveTime)
      (bind _asbp_board_game_instance (Utilities|Casting|CastToBP_BoardGameInstance (Game|GetGameInstance)))
      (Variables|/Game/Board/BP_BoardGameInstance.BP_BoardGameInstance_C|SetfromMinigame _asbp_board_game_instance true)
      (Class|GameplayStatics|SetForceDisableSplitscreen false)
      (Game|OpenLevel(byName) (Utilities|String|StringToName (Utilities|Array|Get(acopy) (Variables|Default|GetMinigames) (Math|Random|RandomIntegerinRange 0 2)))))))

(event Custom|EndGame
  (bind _outactors (Actor|GetAllActorsOfClass "/Game/Board/BP_CutsceneCheckPoint.BP_CutsceneCheckPoint_C"))
  (Variables|Default|Setpoints _outactors)
  (bind _returnvalue (Actor|GetActorOfClass "/Script/CinematicCamera.CineCameraActor"))
  (Variables|Default|SetfinalCamera _returnvalue)
  (bind _returnvalue_2 (UserInterface|CreateWidget "/Game/Board/UI/WidgetDialog.WidgetDialog_C" (Game|GetPlayerController 0)))
  (bind _output_get (Variables|Default|SetDRef _returnvalue_2))
  (UserInterface|Viewport|AddtoViewport _output_get 0)
  (|PlayEndgameDialog (Variables|Default|GetDRef) (Variables|Default|GetturnOrder) (Variables|Default|Getpoints) (Variables|Default|GetfinalCamera) 1.5 0.0
    (:OnFinished
      (Utilities|FlowControl|Delay 1.2)
      (Game|OpenLevel(byObjectReference) "/Game/MainMenu/Main_Menu.Main_Menu"))))

(event EventBeginPlay
  (bind _returnvalue (Actor|GetActorOfClass "/Game/Board/BP_MedalSelector.BP_MedalSelector_C"))
  (Variables|Default|Setselector _returnvalue)
  (Class|GameplayStatics|SetForceDisableSplitscreen true)
  (bind _asbp_board_game_instance (Utilities|Casting|CastToBP_BoardGameInstance (Game|GetGameInstance)))
  (if (Variables|/Game/Board/BP_BoardGameInstance.BP_BoardGameInstance_C|GetfromMinigame _asbp_board_game_instance)
    (Variables|/Game/Board/BP_BoardGameInstance.BP_BoardGameInstance_C|SetfromMinigame _asbp_board_game_instance false)
    (if (Variables|/Game/Board/BP_BoardGameInstance.BP_BoardGameInstance_C|GetfromGamble _asbp_board_game_instance)
      (Variables|/Game/Board/BP_BoardGameInstance.BP_BoardGameInstance_C|SetfromGamble _asbp_board_game_instance false)
      (CallFunction|LoadTime)
      (bind _outactors (Actor|GetAllActorsOfClass "/Game/Board/BP_Character.BP_Character_C"))
      (for _array_element _outactors
        (bind _asbp_character (Utilities|Casting|CastToBP_Character _array_element))
        (if (== (Variables|/Game/Board/BP_Character.BP_Character_C|GetID _asbp_character) (Variables|/Game/Board/BP_BoardGameInstance.BP_BoardGameInstance_C|GetWinnerID _asbp_board_game_instance))
          (Variables|/Game/Board/BP_Character.BP_Character_C|Setdollars _asbp_character (Variables|/Game/Board/BP_BoardGameInstance.BP_BoardGameInstance_C|GetSet_WinMoney _asbp_board_game_instance))
          (Development|PrintString "Completed")
          (CallFunction|StartTurn)
          (bind _returnvalue_2 (UserInterface|CreateWidget "/Game/Board/UI/WidgetHud.WidgetHud_C"))
          (UserInterface|Viewport|AddtoViewport _returnvalue_2 0)
          (if (Utilities|Array|IsEmpty (Variables|Default|GetroundOrder))
            (Utilities|FlowControl|Delay 1.0)
            (CallFunction|EndRound))))
      (else
        (CallFunction|LoadTime)
        (bind _outactors_2 (Actor|GetAllActorsOfClass "/Game/Board/BP_Character.BP_Character_C"))
        (for _array_element_2 _outactors_2
          (bind _asbp_character_2 (Utilities|Casting|CastToBP_Character _array_element_2))
          (if (== (Variables|/Game/Board/BP_Character.BP_Character_C|GetID _asbp_character_2) (Variables|/Game/Board/BP_BoardGameInstance.BP_BoardGameInstance_C|GetWinnerID _asbp_board_game_instance))
            (Default|AddDollars _asbp_character_2 (Variables|/Game/Board/BP_BoardGameInstance.BP_BoardGameInstance_C|GetSet_WinMoney _asbp_board_game_instance))
            (CallFunction|SaveTime))
          (if (<= (Variables|Default|Getrounds) 0)
            (CallFunction|EndGame)
            (else
              (CallFunction|InitiateRound)
              (bind _returnvalue_3 (UserInterface|CreateWidget "/Game/Board/UI/WidgetHud.WidgetHud_C"))
              (UserInterface|Viewport|AddtoViewport _returnvalue_3 0))))))
    (else
      (bind _outactors_3 (Actor|GetAllActorsOfClass "/Game/Board/BP_Character.BP_Character_C"))
      (Variables|Default|SetturnOrder _outactors_3)
      (Default|MedalChosen (Variables|Default|Getselector))
      (CallFunction|InitiateRound)
      (bind _returnvalue_4 (UserInterface|CreateWidget "/Game/Board/UI/WidgetHud.WidgetHud_C"))
      (UserInterface|Viewport|AddtoViewport _returnvalue_4 0))))

(fn ConstructionScript)

(fn LoadTime
  (bind _returnvalue (SaveGame|LoadGamefromSlot "PartySave"))
  (bind _asboard_game_save (Utilities|Casting|CastToBoardGameSave _returnvalue))
  (bind _output_get (Variables|Default|SetLoadData _asboard_game_save))
  (bind _output_get_2 (Variables|/Game/Board/BP_MedalSelector.BP_MedalSelector_C|SetMedal%20Space (Variables|Default|Getselector) (Variables|/Game/Board/BoardGameSave.BoardGameSave_C|Getmedalspace _output_get)))
  (Variables|/Game/Board/BP_Spacess.BP_Spacess_C|SetSpaceType _output_get_2 "NewEnumerator4")
  (Rendering|Material|SetMaterial (Variables|/Game/Board/BP_Spacess.BP_Spacess_C|GetCylinder _output_get_2) 0 "/Game/Board/M_BoardSpace_Inst3.M_BoardSpace_Inst3")
  (bind _asbp_board_game_instance (Utilities|Casting|CastToBP_BoardGameInstance (Game|GetGameInstance)))
  (Variables|/Game/Board/BP_BoardGameInstance.BP_BoardGameInstance_C|SetNumberofPlayer _asbp_board_game_instance (Variables|/Game/Board/BoardGameSave.BoardGameSave_C|Getplayernum _output_get))
  (Variables|Default|Setrounds (Variables|/Game/Board/BoardGameSave.BoardGameSave_C|Getrounds _output_get))
  (Variables|Default|SetturnOrder (Variables|/Game/Board/BoardGameSave.BoardGameSave_C|GetturnOrder _output_get))
  (Variables|Default|SetroundOrder (Variables|/Game/Board/BoardGameSave.BoardGameSave_C|GetroundOrder _output_get))
  (for _array_element (Variables|/Game/Board/BoardGameSave.BoardGameSave_C|GetplayerData _output_get)
    (for _array_element_2 (Variables|/Game/Board/BoardGameSave.BoardGameSave_C|GetturnOrder _output_get)
      (bind _asbp_character (Utilities|Casting|CastToBP_Character _array_element_2))
      (if (== (Variables|/Game/Board/BP_Character.BP_Character_C|GetID _asbp_character) (.ID (Utilities|Struct|BreakPlayerData _array_element)))
        (Variables|/Game/Board/BP_Character.BP_Character_C|SetCurrentSpace _asbp_character (.CurrentSpace (Utilities|Struct|BreakPlayerData _array_element)))
        (Variables|/Game/Board/BP_Character.BP_Character_C|Setdollars _asbp_character (.dollars (Utilities|Struct|BreakPlayerData _array_element)))
        (Variables|/Game/Board/BP_Character.BP_Character_C|Setmedals _asbp_character (.medals (Utilities|Struct|BreakPlayerData _array_element)))
        (bind _output_get_3 (Variables|/Game/Board/BP_Character.BP_Character_C|Setcurrentpos _asbp_character (.currentpos (Utilities|Struct|BreakPlayerData _array_element))))
        (Transformation|Teleport _asbp_character _output_get_3 "0, 0, 0")))))

(fn SaveTime
  (Utilities|FlowControl|Sequence
    (:then_0
      (Utilities|IsValid (Variables|Default|GetSaveFileref)
        (:Is%20Not%20Valid
          (bind _returnvalue (SaveGame|CreateSaveGameObject "/Game/Board/BoardGameSave.BoardGameSave_C"))
          (Variables|Default|SetSaveFileref _returnvalue))))
    (:then_1
      (bind _asbp_board_game_instance (Utilities|Casting|CastToBP_BoardGameInstance (Game|GetGameInstance)))
      (Variables|/Game/Board/BoardGameSave.BoardGameSave_C|Setplayernum (Variables|Default|GetSaveFileref) (Variables|/Game/Board/BP_BoardGameInstance.BP_BoardGameInstance_C|GetNumberofPlayer _asbp_board_game_instance))
      (Variables|/Game/Board/BoardGameSave.BoardGameSave_C|Setmedalspace (Variables|Default|GetSaveFileref) (Variables|/Game/Board/BP_MedalSelector.BP_MedalSelector_C|GetMedal%20Space (Variables|Default|Getselector)))
      (Variables|/Game/Board/BoardGameSave.BoardGameSave_C|Setrounds (Variables|Default|GetSaveFileref) (Variables|Default|Getrounds))
      (bind _output_get (Variables|/Game/Board/BoardGameSave.BoardGameSave_C|SetturnOrder (Variables|Default|GetSaveFileref) (Variables|Default|GetturnOrder)))
      (Variables|/Game/Board/BoardGameSave.BoardGameSave_C|SetroundOrder (Variables|Default|GetSaveFileref) (Variables|Default|GetroundOrder))
      (for _array_element _output_get
        (Utilities|Array|AddUnique (Variables|Default|GetSaveData) (Utilities|Struct|MakePlayerData (Variables|/Game/Board/BP_Character.BP_Character_C|GetCurrentSpace _array_element) (Variables|/Game/Board/BP_Character.BP_Character_C|Getdollars _array_element) (Variables|/Game/Board/BP_Character.BP_Character_C|Getmedals _array_element) (Variables|/Game/Board/BP_Character.BP_Character_C|Getcurrentpos _array_element) (Variables|/Game/Board/BP_Character.BP_Character_C|GetID _array_element)))
        (Variables|/Game/Board/BoardGameSave.BoardGameSave_C|SetplayerData (Variables|Default|GetSaveFileref) (Variables|Default|GetSaveData))
        (SaveGame|SaveGametoSlot (Variables|Default|GetSaveFileref) "PartySave")))))