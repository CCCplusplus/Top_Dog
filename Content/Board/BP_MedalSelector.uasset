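; BP_MedalSelector picks which board space holds the Medal in a board game.
; MedalChosen scans ValidSpaces and, if no medal is flagged, turns a random space into a Medal space, swaps its cylinder material and removes it from the pool.
; ChangeMedal first removes the current MedalSpace from the pool, then repeats that logic.
; Neither event resets IsThereMedal or restores the previous space's type or material.
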(event Custom|MedalChosen
  (bind _valid_spaces (Variables|Default|GetValid_Spaces))
  (for _array_element _valid_spaces
    (switch Utilities|FlowControl|Switch|SwitchonE_SpaceType (Variables|/Game/Board/BP_Spacess.BP_Spacess_C|GetSpaceType _array_element)
      (:NewEnumerator4
        (bind _output_get (Variables|Default|Setis%20there%20medal? true)))))
  (if (not _output_get)
    (bind _output_get_2 (Variables|Default|SetMedal%20Space (Utilities|Array|Get(acopy) _valid_spaces (Math|Random|RandomInteger (Utilities|Array|Length _valid_spaces)))))
    (Variables|/Game/Board/BP_Spacess.BP_Spacess_C|SetSpaceType _output_get_2 "NewEnumerator4")
    (Rendering|Material|SetMaterial (Variables|/Game/Board/BP_Spacess.BP_Spacess_C|GetCylinder _output_get_2) 0 "/Game/Board/M_BoardSpace_Inst3.M_BoardSpace_Inst3")
    (Utilities|Array|RemoveItem (Variables|Default|GetValid_Spaces) (Variables|Default|GetMedal%20Space))))

(event Custom|ChangeMedal
  (bind _valid_spaces (Variables|Default|GetValid_Spaces))
  (Utilities|Array|RemoveItem (Variables|Default|GetValid_Spaces) (Variables|Default|GetMedal%20Space))
  (for _array_element _valid_spaces
    (switch Utilities|FlowControl|Switch|SwitchonE_SpaceType (Variables|/Game/Board/BP_Spacess.BP_Spacess_C|GetSpaceType _array_element)
      (:NewEnumerator4
        (bind _output_get (Variables|Default|Setis%20there%20medal? true)))))
  (if (not _output_get)
    (bind _output_get_2 (Variables|Default|SetMedal%20Space (Utilities|Array|Get(acopy) _valid_spaces (Math|Random|RandomInteger (Utilities|Array|Length _valid_spaces)))))
    (Variables|/Game/Board/BP_Spacess.BP_Spacess_C|SetSpaceType _output_get_2 "NewEnumerator4")
    (Rendering|Material|SetMaterial (Variables|/Game/Board/BP_Spacess.BP_Spacess_C|GetCylinder _output_get_2) 0 "/Game/Board/M_BoardSpace_Inst3.M_BoardSpace_Inst3")
    (Utilities|Array|RemoveItem (Variables|Default|GetValid_Spaces) (Variables|Default|GetMedal%20Space))))

(fn ConstructionScript)