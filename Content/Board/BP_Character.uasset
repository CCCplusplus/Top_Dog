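; Board game pawn for one player slot, possessed by a local controller or flagged as a bot based on player count.
; A die widget's roll sets the moves, walked space by space with AI MoveTo; forks prompt a path widget, or bots choose randomly.
; Shop and Medal are placeholders that consume no move.
; The landing space changes dollars, teleports randomly, prints a mob message, or saves state and opens blackjack, with dispatchers signalling turn end.
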(event Custom|MoveToSpace
  (params (Current_Space :type BP%20Spacess%20Object%20Reference))
  (bind _returnvalue (Game|GetPlayerController 0))
  (bind _nextspace (Variables|/Game/Board/BP_Spacess.BP_Spacess_C|GetNextSpace Current_Space))
  (bind _output (Utilities|Array|Get(acopy) _nextspace))
  ;[1 1 1] Move To Space
  (if (>= (Utilities|Array|Length _nextspace) 2)
    (if (Variables|Default|GetisBot)
      (CallFunction|PathChosen)
      (else
        (bind _returnvalue_2 (UserInterface|CreateWidget "/Game/Board/UI/WidgetPathSelect.WidgetPathSelect_C" _returnvalue self))
        (bind _output_get (Variables|Default|Setchoosewidget _returnvalue_2))
        (UserInterface|Viewport|AddtoViewport _returnvalue_2 0)
        (Input|SetInputModeUIOnly _returnvalue (Variables|Default|Getchoosewidget) "DoNotLock" false)))
    (else
      (Variables|Default|SetCurrentSpace _output)
      (AI|AIMoveTo self "0, 0, 0" _output 5.0 false
        (:OnSuccess
          (switch Utilities|FlowControl|Switch|SwitchonE_SpaceType (Variables|/Game/Board/BP_Spacess.BP_Spacess_C|GetSpaceType (Variables|Default|GetCurrentSpace))
            (:NewEnumerator0
              (CallFunction|BasicSpace))
            (:NewEnumerator1
              (CallFunction|BasicSpace))
            (:NewEnumerator2
              (CallFunction|BasicSpace))
            (:NewEnumerator3
              (Development|PrintString "This should be a shop")
              (Utilities|FlowControl|Delay 0.5)
              (CallFunction|MovetoSpace (Variables|Default|GetCurrentSpace)))
            (:NewEnumerator4
              (Development|PrintString "This should be a medal")
              (Utilities|FlowControl|Delay 0.5)
              (CallFunction|MovetoSpace (Variables|Default|GetCurrentSpace)))
            (:NewEnumerator5
              (CallFunction|BasicSpace))
            (:NewEnumerator6
              (CallFunction|BasicSpace))))))))

(event Custom|TurnEnded
  (bind _as_widget_die_roll (Variables|Default|GetAs%20Widget%20Die%20Roll))
  (bind _randomspaces (Variables|Default|GetRandomspaces))
  ;[1 1 1] Turn end
  (EventDispatchers|UnbindallEventsfromOnRollStop _as_widget_die_roll)
  (Widget|SetVisibility _as_widget_die_roll "Hidden")
  (Utilities|FlowControl|Delay 2.0)
  (Utilities|FlowControl|Sequence
    (:then_0
      (switch Utilities|FlowControl|Switch|SwitchonE_SpaceType (Variables|/Game/Board/BP_Spacess.BP_Spacess_C|GetSpaceType (Variables|Default|GetCurrentSpace))
        (:NewEnumerator0
          (CallFunction|AddDollars 30)
          (Variables|Default|Setcurrentpos (Transformation|GetWorldLocation (Variables|/Script/Engine.Actor|GetRootComponent (Variables|Default|GetCurrentSpace))) :!label _label))
        (:NewEnumerator1
          (CallFunction|AddDollars -30)
          (goto _label))
        (:NewEnumerator2
          (bind _output_get (Variables|Default|SetCurrentSpace (Utilities|Array|Get(acopy) _randomspaces (Math|Random|RandomInteger (Utilities|Array|Length _randomspaces)))))
          (Development|PrintString (Utilities|GetDisplayName _output_get))
          (CallFunction|Movetime self)
          (goto _label))
        (:NewEnumerator5
          (Development|PrintString "Mob Time")
          (goto _label))
        (:NewEnumerator6
          (Variables|Default|Setcurrentpos (Transformation|GetWorldLocation (Variables|/Script/Engine.Actor|GetRootComponent (Variables|Default|GetCurrentSpace))))
          (bind _asbp_board_game_instance (Utilities|Casting|CastToBP_BoardGameInstance (Game|GetGameInstance)))
          (Variables|/Game/Board/BP_BoardGameInstance.BP_BoardGameInstance_C|SetfromMinigame _asbp_board_game_instance true)
          (Variables|/Game/Board/BP_BoardGameInstance.BP_BoardGameInstance_C|SetMoney _asbp_board_game_instance (Math|Conversions|ToFloat(Integer) (Variables|Default|Getdollars)))
          (Variables|/Game/Board/BP_BoardGameInstance.BP_BoardGameInstance_C|SetWinnerID _asbp_board_game_instance (Variables|Default|GetID))
          (Variables|/Game/Board/BP_BoardGameInstance.BP_BoardGameInstance_C|SetfromGamble _asbp_board_game_instance true)
          (bind _asbp_board_game_mode (Utilities|Casting|CastToBP_BoardGameMode (Game|GetGameMode)))
          (Utilities|Array|RemoveIndex (Variables|/Game/Board/BP_BoardGameMode.BP_BoardGameMode_C|GetroundOrder _asbp_board_game_mode))
          (Default|SaveTime _asbp_board_game_mode)
          (Game|OpenLevel(byName) "BlackJackEntry"))))
    (:then_1
      (Default|CallOnTurnEnded)
      (Default|CallOnDollarsCollected))))

(event Custom|RollDie
  (bind _as_widget_die_roll (Variables|Default|GetAs%20Widget%20Die%20Roll))
  ;[1 1 1] Roll Die
  (Game|Player|SetViewTargetwithBlend (Game|GetPlayerController 0) self 1.0 "VTBlend_Linear" 0.0 false)
  (Widget|SetVisibility _as_widget_die_roll "Visible")
  (Default|OnStartRoll _as_widget_die_roll)
  (if (Variables|Default|GetisBot)
    (Default|BOTDice _as_widget_die_roll))
  (EventDispatchers|BindEventtoOnRollStop _as_widget_die_roll (delegate Custom|RollStopped)))

(event Custom|BasicSpace
  ;[1 1 1] Basic Space
  (bind _result (Math|Integer|DecrementInt (Variables|Default|GetMovesRemaining))
    (:%20%20
      (Rendering|Components|TextRender|SetText (Variables|/Game/Board/UI/WidgetDieRoll.WidgetDieRoll_C|GetRoll (Variables|Default|GetAs%20Widget%20Die%20Roll)) (Utilities|Text|ToText(Integer) _result))
      (if (> _result 0)
        (CallFunction|MovetoSpace (Variables|Default|GetCurrentSpace))
        (else
          (CallFunction|TurnEnded))))))

(event Custom|PathChosen
  (params (way :type Integer))
  ;[1 1 1] Choosing a PAth
  (if (Variables|Default|GetisBot)
    (Variables|Default|Setpath (Math|Random|RandomIntegerinRange 0 1))
    (Variables|Default|SetCurrentSpace (Utilities|Array|Get(acopy) (Variables|/Game/Board/BP_Spacess.BP_Spacess_C|GetNextSpace (Variables|Default|GetCurrentSpace)) (Variables|Default|Getpath)))
    (else
      (Input|SetInputModeGameOnly (Game|GetPlayerController 0) false)
      (Variables|Default|Setpath way)
      (bind _output_get (Variables|Default|SetCurrentSpace (Utilities|Array|Get(acopy) (Variables|/Game/Board/BP_Spacess.BP_Spacess_C|GetNextSpace (Variables|Default|GetCurrentSpace)) (Variables|Default|Getpath))))))
  (AI|AIMoveTo self "0, 0, 0" _output_get 5.0 false
    (:OnSuccess
      (switch Utilities|FlowControl|Switch|SwitchonE_SpaceType (Variables|/Game/Board/BP_Spacess.BP_Spacess_C|GetSpaceType (Variables|Default|GetCurrentSpace))
        (:NewEnumerator0
          (CallFunction|BasicSpace))
        (:NewEnumerator1
          (CallFunction|BasicSpace))
        (:NewEnumerator2
          (CallFunction|BasicSpace))
        (:NewEnumerator3
          (Development|PrintString "This should be a shop")
          (Utilities|FlowControl|Delay 0.5)
          (CallFunction|MovetoSpace (Variables|Default|GetCurrentSpace)))
        (:NewEnumerator4
          (Development|PrintString "This should be a medal")
          (Utilities|FlowControl|Delay 0.5)
          (CallFunction|MovetoSpace (Variables|Default|GetCurrentSpace)))
        (:NewEnumerator5
          (CallFunction|BasicSpace))
        (:NewEnumerator6
          (CallFunction|BasicSpace))))))

(event Custom|RollStopped
  (params (Number :type Integer))
  ;[1 1 1] Roll Die
  (Variables|Default|SetMovesRemaining Number)
  (EventDispatchers|UnbindallEventsfromOnRollStop (Variables|Default|GetAs%20Widget%20Die%20Roll))
  (CallFunction|MovetoSpace (Variables|Default|GetCurrentSpace)))

(event Custom|SelectSpaces
  ;[1 1 1] Random Space Select
  (bind _outactors (Actor|GetAllActorsOfClass "/Game/Board/BP_Spacess.BP_Spacess_C"))
  (bind _output_get (Variables|Default|SetAllSpaces _outactors))
  (for _array_element _output_get
    (switch Utilities|FlowControl|Switch|SwitchonE_SpaceType (Variables|/Game/Board/BP_Spacess.BP_Spacess_C|GetSpaceType _array_element)
      (:NewEnumerator0
        (Utilities|Array|AddUnique (Variables|Default|GetRandomspaces) _array_element))
      (:NewEnumerator1
        (Utilities|Array|AddUnique (Variables|Default|GetRandomspaces) _array_element))
      (:NewEnumerator5
        (Utilities|Array|AddUnique (Variables|Default|GetRandomspaces) _array_element))
      (:NewEnumerator6
        (Utilities|Array|AddUnique (Variables|Default|GetRandomspaces) _array_element)))))

(event Custom|Movetime
  ;[1 1 1] Teleport
  (bind _returnvalue (Transformation|Teleport self (Transformation|GetWorldLocation (Variables|/Script/Engine.Actor|GetRootComponent (Variables|Default|GetCurrentSpace))) "0, 0, 0"))
  (if (not _returnvalue)
    (CallFunction|Movetime self)))

(event EventBeginPlay
  (bind _returnvalue (Game|GetGameInstance))
  ;[1 1 1] Beggin_Play
  (if (== (Variables|Default|GetID) "Player_2")
    (bind _asbp_board_game_instance (Utilities|Casting|CastToBP_BoardGameInstance _returnvalue))
    (if (>= (Variables|/Game/Board/BP_BoardGameInstance.BP_BoardGameInstance_C|GetNumberofPlayer _asbp_board_game_instance) 2)
      (Class|GameplayStatics|CreatePlayer 1)
      (Utilities|FlowControl|Delay 0.2)
      (Pawn|Possess (Game|GetPlayerController 1))
      (else
        (Variables|Default|SetisBot true)))
    (elif (== (Variables|Default|GetID) "Player_3")
      (bind _asbp_board_game_instance_2 (Utilities|Casting|CastToBP_BoardGameInstance _returnvalue))
      (if (>= (Variables|/Game/Board/BP_BoardGameInstance.BP_BoardGameInstance_C|GetNumberofPlayer _asbp_board_game_instance_2) 3)
        (Class|GameplayStatics|CreatePlayer 2)
        (Utilities|FlowControl|Delay 0.2)
        (Pawn|Possess (Game|GetPlayerController 2))
        (else
          (Variables|Default|SetisBot true)))
      (elif (== (Variables|Default|GetID) "Player_4")
        (bind _asbp_board_game_instance_3 (Utilities|Casting|CastToBP_BoardGameInstance _returnvalue))
        (if (== (Variables|/Game/Board/BP_BoardGameInstance.BP_BoardGameInstance_C|GetNumberofPlayer _asbp_board_game_instance_3) 4)
          (Utilities|FlowControl|Delay 0.2)
          (Class|GameplayStatics|CreatePlayer 3)
          (Pawn|Possess (Game|GetPlayerController 3))
          (else
            (Variables|Default|SetisBot true))))))
  (bind _aswidget_die_roll (Utilities|Casting|CastToWidgetDieRoll (UserInterface|GetWidget (Variables|Default|Getw))))
  (Variables|Default|SetAs%20Widget%20Die%20Roll _aswidget_die_roll)
  (CallFunction|SelectSpaces))

(fn ConstructionScript)

(fn AddDollars
  (params (Number :type Integer))
  (if (< (+ (Variables|Default|Getdollars) Number) 0)
    (Variables|Default|Setdollars 0)
    (else
      (Variables|Default|Setdollars (+ (Variables|Default|Getdollars) Number)))))